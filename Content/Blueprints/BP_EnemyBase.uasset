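; Base enemy for turn-based battles, selectable by click through BP_GameMode_Battle, with a selection circle and HP widget.
; TakeDamage spawns a damage number, clamps health and reports death to the game mode.
; AttackPlayer damages the player and sets attack state flags.
; A BP_BossEnemy check in this base class makes the boss periodically summon two base enemies into EnemyArray and hand the turn back instead of attacking.
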(event `self.ReceiveBeginPlay`
  (set `self.CurrentHealth` (`self.MaxHealth`))
  (`KismetSystemLibrary.Delay` 0.1)
  (bind _aswbp_enemy_hp (cast `/Game/Widgets/WBP_EnemyHP` (`WidgetComponent.GetUserWidgetObject` (`self.EnemyHPWidget`))))
  (set `/Game/Widgets/WBP_EnemyHP.EnemyReference` self _aswbp_enemy_hp))

(event `self.ReceiveActorOnClicked`
  (params (ButtonPressed :type "Key Structure"))
  (bind _asbp_game_mode_battle (cast `/Game/Blueprints/BP_GameMode_Battle` (`GameplayStatics.GetGameMode`)))
  (`/Game/Blueprints/BP_GameMode_Battle.SelectEnemyByIndex` _asbp_game_mode_battle (`KismetArrayLibrary.Array_Find` (`/Game/Blueprints/BP_GameMode_Battle.EnemyArray` _asbp_game_mode_battle) self)))

(event `SetSelected`
  (params (NewState :type Boolean))
  (`SceneComponent.SetVisibility` (`self.SelectionCircle`) NewState false))

(fn `AttackPlayer`
  (bind _asbp_game_mode_battle (cast `/Game/Blueprints/BP_GameMode_Battle` (`GameplayStatics.GetGameMode`)))
  (set `/Game/Blueprints/BP_GameMode_Battle.BattleState` "NewEnumerator2" _asbp_game_mode_battle)
  (`KismetSystemLibrary.PrintString` "Enemy Attacks!")
  (bind _asbp_third_person_character (cast `/Game/ThirdPerson/Blueprints/BP_ThirdPersonCharacter` (`GameplayStatics.GetPlayerCharacter` 0)))
  (bind _returnvalue (`GameplayStatics.GetActorOfClass` "/Game/Blueprints/BP_BossEnemy.BP_BossEnemy_C"))
  (bind _returnvalue_2 (== _returnvalue self))
  (if (and _returnvalue_2 (> (`self.AttackCount`) 1))
    (set `self.bIsSummoning` true)
    (bind _asbp_game_mode_battle_2 (cast `/Game/Blueprints/BP_GameMode_Battle` (`GameplayStatics.GetGameMode`)))
    (`/Game/Blueprints/BP_GameMode_Battle.StartPlayerTurn` _asbp_game_mode_battle_2)
    (bind _enemyspawnpoints (`/Game/Blueprints/BP_GameMode_Battle.EnemySpawnPoints` _asbp_game_mode_battle_2))
    (bind _returnvalue_3 (`|SpawnActorFromClass` "BP_EnemyBase_C" (`self.GetTransform` (`|GetArrayItem` _enemyspawnpoints)) "AdjustIfPossibleButDontSpawnIfColliding" "MultiplyWithRoot" null null))
    (`KismetArrayLibrary.Array_Add` (`/Game/Blueprints/BP_GameMode_Battle.EnemyArray` _asbp_game_mode_battle_2) _returnvalue_3)
    (bind _returnvalue_4 (`|SpawnActorFromClass` "BP_EnemyBase_C" (`self.GetTransform` (`|GetArrayItem` _enemyspawnpoints 2)) "AdjustIfPossibleButDontSpawnIfColliding" "MultiplyWithRoot" null null))
    (`KismetArrayLibrary.Array_Add` (`/Game/Blueprints/BP_GameMode_Battle.EnemyArray` _asbp_game_mode_battle_2) _returnvalue_4)
    (set `self.AttackCount` 0)
    (else
      (set `self.bIsAttacking` true)
      (`/Game/ThirdPerson/Blueprints/BP_ThirdPersonCharacter.TakeDamage` _asbp_third_person_character (`self.AttackDamage`))
      (if _returnvalue_2
        (set `self.AttackCount` (+ (`self.AttackCount`) 1))))))

(fn `TakeDamage`
  (params (DamageAmount :type "Float (double-precision)"))
  (`|SpawnActorFromClass` "/Game/Blueprints/BP_DamageAmount.BP_DamageAmount_C" (`KismetMathLibrary.MakeTransform` (`self.K2_GetActorLocation`)) "Undefined" "MultiplyWithRoot" null DamageAmount null)
  (set `self.CurrentHealth` (`KismetMathLibrary.FClamp` (- (`self.CurrentHealth`) DamageAmount) 0.0 (`self.MaxHealth`)))
  (if (<= (`self.CurrentHealth`) 0.0)
    (bind _asbp_game_mode_battle (cast `/Game/Blueprints/BP_GameMode_Battle` (`GameplayStatics.GetGameMode`)))
    (`/Game/Blueprints/BP_GameMode_Battle.OnEnemyKilled` _asbp_game_mode_battle self)
    (set `self.bIsDead` true)))

(fn `UserConstructionScript`)
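; Player controller for the battle mode that lets the player cycle the targeted enemy with the keyboard.
; On BeginPlay it shows the mouse cursor and enables click and mouse-over events.
; D and A step the selected index forward or back through the game mode's EnemyArray, wrapping at the ends, and pass it to SelectEnemyByIndex on BP_GameMode_Battle, which holds the selection state.
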(event `self.ReceiveBeginPlay`
  (set `self.bShowMouseCursor` true)
  (set `self.bEnableClickEvents` true)
  (set `self.bEnableMouseOverEvents` true))

(event `Key|D`
  (params (Key :type "Key Structure"))
  (:`Pressed`
    (bind _asbp_game_mode_battle (cast `/Game/Blueprints/BP_GameMode_Battle` (`GameplayStatics.GetGameMode`)))
    (bind _output_get (set `self.NewIndex` (+ (`/Game/Blueprints/BP_GameMode_Battle.CurrentSelectedIndex` _asbp_game_mode_battle) 1)))
    (if (>= _output_get (`KismetArrayLibrary.Array_Length` (`/Game/Blueprints/BP_GameMode_Battle.EnemyArray` _asbp_game_mode_battle)))
      (bind _output_get_2 (set `self.NewIndex` 0))
      (else
        (set `self.NewIndex` (`self.NewIndex`))))
    (`/Game/Blueprints/BP_GameMode_Battle.SelectEnemyByIndex` _asbp_game_mode_battle _output_get_2)))

(event `Key|A`
  (params (Key :type "Key Structure"))
  (:`Pressed`
    (bind _asbp_game_mode_battle (cast `/Game/Blueprints/BP_GameMode_Battle` (`GameplayStatics.GetGameMode`)))
    (bind _output_get (set `self.NewIndex` (- (`/Game/Blueprints/BP_GameMode_Battle.CurrentSelectedIndex` _asbp_game_mode_battle) 1)))
    (if (< _output_get 0)
      (bind _output_get_2 (set `self.NewIndex` (- (`KismetArrayLibrary.Array_Length` (`/Game/Blueprints/BP_GameMode_Battle.EnemyArray` _asbp_game_mode_battle)) 1)))
      (else
        (set `self.NewIndex` (`self.NewIndex`))))
    (`/Game/Blueprints/BP_GameMode_Battle.SelectEnemyByIndex` _asbp_game_mode_battle _output_get_2)))

(fn `UserConstructionScript`)
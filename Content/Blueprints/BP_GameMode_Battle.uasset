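; Game mode for a turn-based battle with typed skills, running two three-enemy waves and a boss before loading the Win level.
; A battle-state enum gates menu commands: attack damages the selected enemy, defend passes, and skills go through TypingManager, whose callback spawns the skill actor.
; Enemies attack sequentially through a delayed self-calling event, then the player menu returns.
; Kills advance waves and reselect targets; Defeat loads GameOver.
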(event `self.ReceiveBeginPlay`
  (bind _returnvalue (`GameplayStatics.GetActorOfClass` "/Game/Blueprints/skills/TypingManager.TypingManager_C"))
  (set `self.typingMangerRef` _returnvalue)
  (add `/Game/Blueprints/skills/TypingManager.FinishedTyping` (`self.typingMangerRef`) (delegate `skillAttack`))
  (bind _outactors (`GameplayStatics.GetAllActorsOfClass` "/Script/Engine.TargetPoint"))
  (set `self.EnemySpawnPoints` _outactors)
  (`self.SpawnWave`)
  (`self.StartPlayerTurn`)
  (bind _returnvalue_2 (`|CreateWidget` "/Game/Widgets/WBP_BattleUI.WBP_BattleUI_C"))
  (`UserWidget.AddToViewport` _returnvalue_2 0)
  (`self.SelectEnemyByIndex` 1))

(event `EnemyAttackLoop`
  (`KismetSystemLibrary.PrintString` "EnemyLoop Start")
  (if (>= (`self.EnemyTurnIndex`) (`KismetArrayLibrary.Array_Length` (`self.EnemyArray`)))
    (`KismetSystemLibrary.PrintString` "Player Turn")
    (`self.StartPlayerTurn`)
    (else
      (bind _output_get (set `self.TempEnemy` (`|GetArrayItem` (`self.EnemyArray`) (`self.EnemyTurnIndex`))))
      (`/Engine/EditorBlueprintResources/StandardMacros.IsValid` _output_get
        (:`Is Valid`
          (`/Game/Blueprints/BP_EnemyBase.AttackPlayer` (`self.TempEnemy`))
          (set `self.EnemyTurnIndex` (+ (`self.EnemyTurnIndex`) 1))
          (`KismetSystemLibrary.Delay` 2.1)
          (`self.EnemyAttackLoop`))))))

(event `skillAttack`
  (params (skill :type "/Game/Blueprints/skills/BP_skillBase Class Reference") (success :type Boolean))
  (bind _returnvalue (`GameplayStatics.GetPlayerCharacter` 0))
  (bind (_skillname _mpcost _basedmg _timelimit _multiplier _gamemode _mpcostreduce _target _projectilespeed) (defaults `Object` skill))
  (bind _returnvalue_2 (`|SpawnActorFromClass` skill (`KismetMathLibrary.Conv_VectorToTransform` (+ (`self.K2_GetActorLocation` _returnvalue) (50.0 0.0 0.0))) "Undefined" "MultiplyWithRoot" _returnvalue _skillname _mpcost _basedmg _timelimit _multiplier _mpcostreduce _projectilespeed null))
  (`/Game/Blueprints/skills/BP_skillBase.OnTypingFinish` _returnvalue_2 success)
  (if (!= (`KismetTextLibrary.Conv_TextToString` _skillname) "Heal")
    (`/Game/Blueprints/skills/BP_skillBase.setvelocity` _returnvalue_2 (`self.SelectedEnemy`))
    (else
      (`/Game/Blueprints/skills/BP_skillBase.Heal` _returnvalue_2))))

(event `OnEnemyKilled`
  (params (DeadEnemy :type "/Game/Blueprints/BP_EnemyBase Object Reference"))
  (`KismetArrayLibrary.Array_RemoveItem` (`self.EnemyArray`) DeadEnemy)
  (if (== (`KismetArrayLibrary.Array_Length` (`self.EnemyArray`)) 0)
    (set `self.CurrentWave` (+ (`self.CurrentWave`) 1))
    (`KismetSystemLibrary.Delay` 2.0)
    (`self.SpawnWave`)
    (`self.SelectEnemyByIndex` 0)
    (else
      (`self.SelectEnemyByIndex` 0))))

(event `/Game/Blueprints/skills/BPI_TakeDMGCall.onFinishedTyping`
  (params (DMGamount :type "Float (double-precision)"))
  (`/Game/Blueprints/BP_EnemyBase.TakeDamage` (`self.SelectedEnemy`) DMGamount)
  (`self.StartEnemyTurn`))

(event `SpawnWave`
  (`KismetArrayLibrary.Array_Clear` (`self.EnemyArray`))
  (`KismetSystemLibrary.PrintString` (`KismetStringLibrary.Concat_StrStr` "Wave" "_" (`KismetStringLibrary.Conv_IntToString` (+ (`self.CurrentWave`) 1))) true true (struct :`R` 0.005055 :`B` 0.48 :`A` 1.0))
  (switch `int` (`self.CurrentWave`)
    (:`0`
      (for _index (range 3)
        (bind _returnvalue (`|SpawnActorFromClass` "/Game/Blueprints/BP_EnemyBase.BP_EnemyBase_C" (`self.GetTransform` (`|GetArrayItem` (`self.EnemySpawnPoints`) _index)) "AlwaysSpawn" "MultiplyWithRoot" null null))
        (`KismetArrayLibrary.Array_Add` (`self.EnemyArray`) _returnvalue)))
    (:`1`
      (for _index_2 (range 3)
        (bind _returnvalue_2 (`|SpawnActorFromClass` "/Game/Blueprints/BP_EnemyElite.BP_EnemyElite_C" (`self.GetTransform` (`|GetArrayItem` (`self.EnemySpawnPoints`) _index_2)) "AlwaysSpawn" "MultiplyWithRoot" null null))
        (`KismetArrayLibrary.Array_Add` (`self.EnemyArray`) _returnvalue_2)))
    (:`2`
      (for _index_3 (range 1 2)
        (bind _returnvalue_3 (`|SpawnActorFromClass` "/Game/Blueprints/BP_BossEnemy.BP_BossEnemy_C" (`self.GetTransform` (`|GetArrayItem` (`self.EnemySpawnPoints`) _index_3)) "AlwaysSpawn" "MultiplyWithRoot" null null))
        (`KismetArrayLibrary.Array_Add` (`self.EnemyArray`) _returnvalue_3)
        (bind _asbp_third_person_character (cast `/Game/ThirdPerson/Blueprints/BP_ThirdPersonCharacter` (`GameplayStatics.GetPlayerCharacter` 0)))
        (`/Game/ThirdPerson/Blueprints/BP_ThirdPersonCharacter.ZoomOutForBoss` _asbp_third_person_character)))
    (:`3`
      (`GameplayStatics.OpenLevel` "Win"))))

(fn `Defeat`
  (set `self.BattleState` "NewEnumerator4")
  (`KismetSystemLibrary.PrintString` "GAME OVER" true true (struct :`R` 0.856 :`A` 1.0))
  (`GameplayStatics.OpenLevel` "GameOver"))

(fn `DoAttack`
  (set `self.BattleState` "NewEnumerator2")
  (`/Engine/EditorBlueprintResources/StandardMacros.IsValid` (`self.SelectedEnemy`)
    (:`Is Valid`
      (`/Game/Blueprints/BP_EnemyBase.TakeDamage` (`self.SelectedEnemy`) 100.0)
      (`self.StartEnemyTurn`))))

(fn `DoEndTurn`
  (set `self.BattleState` "NewEnumerator2")
  (`self.StartEnemyTurn`))

(fn `DoSkill`
  (params (Skillindex :type Integer))
  (set `self.BattleState` "NewEnumerator2")
  (`/Engine/EditorBlueprintResources/StandardMacros.IsValid` (`self.SelectedEnemy`)
    (:`Is Valid`
      (bind _asbp_third_person_character (cast `/Game/ThirdPerson/Blueprints/BP_ThirdPersonCharacter` (`GameplayStatics.GetPlayerCharacter` 0)))
      (bind _output_get (set `self.PendingSkill` (`|GetArrayItem` (`/Game/ThirdPerson/Blueprints/BP_ThirdPersonCharacter.Skills` _asbp_third_person_character) Skillindex)))
      (`/Game/Blueprints/skills/TypingManager.StartTyping` (`self.typingMangerRef`) _output_get))))

(fn `OnEnemyKilled1`
  (params (DeadEnemy :type "/Game/Blueprints/BP_EnemyBase Object Reference"))
  (`KismetArrayLibrary.Array_RemoveItem` (`self.EnemyArray`) DeadEnemy)
  (if (== (`KismetArrayLibrary.Array_Length` (`self.EnemyArray`)) 0)
    (set `self.CurrentWave` (+ (`self.CurrentWave`) 1))
    (`self.SpawnWave1`)
    (`self.SelectEnemyByIndex` 0)
    (else
      (`self.SelectEnemyByIndex` 0))))

(fn `OpenSkillMenu`
  (`self.DoSkill` 0))

(fn `SelectCommand`
  (params (CommandType :type "/Game/Blueprints/E_PlayerCommand Enum" :default "NewEnumerator0") (`skill index` :type Integer))
  (bind _battlemenuref (`self.BattleMenuRef`))
  (if (`|EnumEquality` (`self.BattleState`) "NewEnumerator0")
    (bind _output_get (set `self.SelectedCommand` (`local.CommandType`)))
    (switch `/Game/Blueprints/E_PlayerCommand` _output_get
      (:`NewEnumerator0`
        (`/Engine/EditorBlueprintResources/StandardMacros.IsValid` (`self.SelectedEnemy`)
          (:`Is Valid`
            (`Widget.RemoveFromParent` _battlemenuref)
            (set `self.BattleState` "NewEnumerator2")
            (`self.DoAttack`))))
      (:`NewEnumerator1`
        (`/Engine/EditorBlueprintResources/StandardMacros.IsValid` (`self.SelectedEnemy`)
          (:`Is Valid`
            (`Widget.RemoveFromParent` _battlemenuref)
            (set `self.BattleState` "NewEnumerator2")
            (`self.DoSkill` `skill index`))))
      (:`NewEnumerator2`
        (`Widget.RemoveFromParent` _battlemenuref)
        (set `self.BattleState` "NewEnumerator2")
        (`self.DoEndTurn`)))))

(fn `SelectEnemyByIndex`
  (params (Index :type Integer))
  (bind _selectedenemy (`self.SelectedEnemy`))
  (if (and (>= Index 0) (< Index (`KismetArrayLibrary.Array_Length` (`self.EnemyArray`))))
    (`/Engine/EditorBlueprintResources/StandardMacros.IsValid` _selectedenemy
      (:`Is Valid`
        (`/Game/Blueprints/BP_EnemyBase.SetSelected` _selectedenemy false))
      (:`Is Not Valid`
        _))
    (bind _output_get (set `self.CurrentSelectedIndex` (`local.Index`)))
    (set `self.SelectedEnemy` (`|GetArrayItem` (`self.EnemyArray`) _output_get))
    (`/Game/Blueprints/BP_EnemyBase.SetSelected` _selectedenemy true)
    (`KismetSystemLibrary.PrintString` "Selected!")))

(fn `ShowBattleMenu`
  (bind _returnvalue (`|CreateWidget` "/Game/Widgets/WBP_BattleMenu.WBP_BattleMenu_C" (`GameplayStatics.GetPlayerController` 0)))
  (bind _output_get (set `self.BattleMenuRef` _returnvalue))
  (`UserWidget.AddToViewport` _output_get 0))

(fn `SpawnWave1`
  (`KismetArrayLibrary.Array_Clear` (`self.EnemyArray`))
  (`KismetSystemLibrary.PrintString` (`KismetStringLibrary.Concat_StrStr` "Wave" "_" (`KismetStringLibrary.Conv_IntToString` (+ (`self.CurrentWave`) 1))) true true (struct :`R` 0.005055 :`B` 0.48 :`A` 1.0))
  (switch `int` (`self.CurrentWave`)
    (:`0`
      (for _index (range 3)
        (bind _returnvalue (`|SpawnActorFromClass` "/Game/Blueprints/BP_EnemyBase.BP_EnemyBase_C" (`self.GetTransform` (`|GetArrayItem` (`self.EnemySpawnPoints`) _index)) "AlwaysSpawn" "MultiplyWithRoot" null null))
        (`KismetArrayLibrary.Array_Add` (`self.EnemyArray`) _returnvalue)))
    (:`1`
      (for _index_2 (range 3)
        (bind _returnvalue_2 (`|SpawnActorFromClass` "/Game/Blueprints/BP_EnemyElite.BP_EnemyElite_C" (`self.GetTransform` (`|GetArrayItem` (`self.EnemySpawnPoints`) _index_2)) "AlwaysSpawn" "MultiplyWithRoot" null null))
        (`KismetArrayLibrary.Array_Add` (`self.EnemyArray`) _returnvalue_2)))
    (:`2`
      (for _index_3 (range 1 2)
        (bind _returnvalue_3 (`|SpawnActorFromClass` "/Game/Blueprints/BP_BossEnemy.BP_BossEnemy_C" (`self.GetTransform` (`|GetArrayItem` (`self.EnemySpawnPoints`) _index_3)) "AlwaysSpawn" "MultiplyWithRoot" null null))
        (`KismetArrayLibrary.Array_Add` (`self.EnemyArray`) _returnvalue_3)
        (bind _asbp_third_person_character (cast `/Game/ThirdPerson/Blueprints/BP_ThirdPersonCharacter` (`GameplayStatics.GetPlayerCharacter` 0)))
        (`/Game/ThirdPerson/Blueprints/BP_ThirdPersonCharacter.ZoomOutForBoss` _asbp_third_person_character)))
    (:`3`
      (`GameplayStatics.OpenLevel` "Win"))))

(fn `StartEnemyTurn`
  (set `self.BattleState` "NewEnumerator1")
  (set `self.EnemyTurnIndex` 0)
  (`self.EnemyAttackLoop`))

(fn `StartPlayerTurn`
  (set `self.BattleState` "NewEnumerator0")
  (bind _returnvalue (`|CreateWidget` "/Game/Widgets/WBP_BattleMenu.WBP_BattleMenu_C" (`GameplayStatics.GetPlayerController` 0)))
  (bind _output_get (set `self.BattleMenuRef` _returnvalue))
  (`UserWidget.AddToViewport` _output_get 0))

(fn `UserConstructionScript`)
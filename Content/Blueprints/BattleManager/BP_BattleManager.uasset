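; BP_BattleManager is an actor that sets up a battle at BeginPlay by spawning the camera, enemies and combat character.
; It spawns a spinning camera at its root and provides a function, not called within this Blueprint, that blends the player view to it.
; Each of five enemy spawn points rolls against its ChangeArray threshold to spawn an AI_Master into EnemyArray.
; One CC_Master spawns at P1 and joins AllyArray.
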(event `self.ReceiveBeginPlay`
  (`self.SpawnCameras`)
  (`self.SpawnEnemies`)
  (`self.SpawnCombatCharacters`))

(fn `SpawnCameras`
  (bind _returnvalue (`|SpawnActorFromClass` "/Game/Blueprints/Cameras/BP_SpinningCamera.BP_SpinningCamera_C" (`SceneComponent.K2_GetComponentToWorld` (`self.DefaultSceneRoot`)) "AlwaysSpawn" "MultiplyWithRoot" null null))
  (set `self.SpinningCamera` _returnvalue))

(fn `SpawnCombatCharacters`
  (bind _p1 (`self.P1`))
  (bind _returnvalue (`|SpawnActorFromClass` "/Game/Blueprints/CombatCharacter/CC_Master.CC_Master_C" (`KismetMathLibrary.MakeTransform` (`SceneComponent.K2_GetComponentLocation` _p1) (`SceneComponent.K2_GetComponentRotation` _p1)) "AlwaysSpawn" "MultiplyWithRoot" null null))
  (`KismetArrayLibrary.Array_Add` (`self.AllyArray`) _returnvalue))

(fn `SpawnEnemies`
  (bind _output_get (set `self.EnemySpawnLocation` (`|MakeArray` (`self.E1`) (`self.E2`) (`self.E3`) (`self.E4`) (`self.E5`))))
  (for (_array_element _array_index) _output_get
    (bind _output_get_2 (set `self.changeValue` (`KismetMathLibrary.RandomFloatInRange` 0.0 1.0)))
    (if (< _output_get_2 (`|GetArrayItem` (`self.ChangeArray`) _array_index))
      (bind _returnvalue (`|SpawnActorFromClass` "/Game/Blueprints/AI/AI_Master.AI_Master_C" (`KismetMathLibrary.MakeTransform` (`SceneComponent.K2_GetComponentLocation` _array_element) (`SceneComponent.K2_GetComponentRotation` _array_element)) "AlwaysSpawn" "MultiplyWithRoot" null null))
      (`KismetArrayLibrary.Array_Add` (`self.EnemyArray`) _returnvalue)
      (`KismetSystemLibrary.PrintString` (`KismetSystemLibrary.GetDisplayName` _returnvalue)))))

(fn `TransitionToSpinningCamera`
  (`PlayerController.SetViewTargetWithBlend` (`GameplayStatics.GetPlayerController` 0) (`self.SpinningCamera`) 2.0 "VTBlend_Linear" 0.0 false))

(fn `UserConstructionScript`)
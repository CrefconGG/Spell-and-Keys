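; BP_DamageAmount is an actor that shows a floating damage number in the world.
; On BeginPlay it passes DamageAmount to its WBP_FloatingDamageNumber widget and picks an end point above its spawn location with slight random sideways jitter.
; A timeline lerps the actor to that point, then destroys it when finished.
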(event `self.ReceiveBeginPlay`
  (bind _aswbp_floating_damage_number (cast `/Game/Widgets/WBP_FloatingDamageNumber` (`WidgetComponent.GetWidget` (`self.Widget`))))
  (set `/Game/Widgets/WBP_FloatingDamageNumber.DamageAmount` (`self.DamageAmount`) _aswbp_floating_damage_number)
  (bind _output_get (set `self.StartLocation` (`self.K2_GetActorLocation`)))
  (set `self.EndLocation` (+ _output_get (`KismetMathLibrary.MakeVector` (`KismetMathLibrary.RandomFloatInRange` -5.0 5.0) (`KismetMathLibrary.RandomFloatInRange` -5.0 5.0) (`KismetMathLibrary.RandomFloatInRange` 25.0 35.0))))
  (bind (_direction _newtrack_0) (`Timeline|Timeline`)
    (:`Update`
      (`self.K2_SetActorLocation` (`KismetMathLibrary.VLerp` (`self.StartLocation`) (`self.EndLocation`) _newtrack_0)))
    (:`Finished`
      (`self.K2_DestroyActor`))))

(fn `UserConstructionScript`)
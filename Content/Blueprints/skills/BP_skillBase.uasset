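; Base skill actor for a typing-driven combat system, with projectile movement and a box collision that ignores its owner.
; A successful typing result lowers the MP cost and multiplies base damage; the player character is charged MP either way.
; Setvelocity aims the projectile slightly above a target's origin, and a hit passes damage to the GameMode before destroying the actor.
; ActivateSkill only prints the skill name.
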(event `self.ReceiveBeginPlay`
  (`PrimitiveComponent.IgnoreActorWhenMoving` (`self.BoxCollision`) (`self.GetOwner`) true))

(event `self.BoxCollision.OnComponentHit`
  (params (HitComponent :type "PrimitiveComponent Object Reference") (OtherActor :type "Actor Object Reference") (OtherComp :type "PrimitiveComponent Object Reference") (NormalImpulse :type "Vector Structure") (Hit :type "HitResult Structure (by ref)"))
  (message `/Game/Blueprints/skills/BPI_TakeDMGCall.onFinishedTyping` (`GameplayStatics.GetGameMode`) (`self.BaseDMG`))
  (`self.K2_DestroyActor`))

(fn `ActivateSkill`
  (params (TypingManagerRef :type "/Game/Blueprints/skills/TypingManager Object Reference"))
  (`KismetSystemLibrary.PrintString` (`KismetTextLibrary.Conv_TextToString` (`self.SkillName`)) true true (struct :`R` 1.0 :`G` 0.892438 :`A` 1.0)))

(fn `consumePlayerMP`
  (`KismetSystemLibrary.PrintString` (`KismetStringLibrary.Conv_IntToString` (`self.MPCost`)) true true (struct :`R` 1.0 :`G` 0.780766 :`A` 1.0))
  (bind _asbp_third_person_character (cast `/Game/ThirdPerson/Blueprints/BP_ThirdPersonCharacter` (`GameplayStatics.GetPlayerCharacter` 0))
    (:`then`
      (`/Game/ThirdPerson/Blueprints/BP_ThirdPersonCharacter.consumeMP` _asbp_third_person_character (`self.MPCost`)))
    (:`CastFailed`
      (`KismetSystemLibrary.PrintString` "ConsumeBP casting failed"))))

(fn `OnTypingFinish`
  (params (Success :type Boolean))
  (if Success
    (set `self.MPCost` (- (`self.MPCost`) (`self.MPcostReduce`)))
    (set `self.BaseDMG` (* (`self.Multiplier`) (`self.BaseDMG`))))
  (`self.consumePlayerMP`))

(fn `setvelocity`
  (params (target :type "Actor Object Reference"))
  (returns (newVelocity :type "Vector Structure"))
  (bind _returnvalue (* (`KismetMathLibrary.GetDirectionUnitVector` (`self.K2_GetActorLocation`) (+ (`self.K2_GetActorLocation` target) (0.0 0.0 100.0))) (`self.projectileSpeed`)))
  (`ProjectileMovementComponent.SetVelocityInLocalSpace` (`self.ProjectileMovement`) _returnvalue)
  (return _returnvalue))

(fn `UserConstructionScript`)
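; Ice lance skill projectile, a child Blueprint that adjusts launch velocity and adds impact effects.
; Its Setvelocity override subtracts 100 on Z from the parent's result and applies it to ProjectileMovement in local space, biasing the lance downward.
; When BoxCollision hits, it spawns a magic-area Niagara effect at the hit point and a hammer-impact effect with no location set.
; The graph itself applies no damage.
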(event `self.BoxCollision.OnComponentHit`
  (params (HitComponent :type "PrimitiveComponent Object Reference") (OtherActor :type "Actor Object Reference") (OtherComp :type "PrimitiveComponent Object Reference") (NormalImpulse :type "Vector Structure") (Hit :type "HitResult Structure (by ref)"))
  (`NiagaraFunctionLibrary.SpawnSystemAtLocation` "/Game/Mixed_Magic_VFX_Pack/VFX/NS_Big_Hammer_Impact.NS_Big_Hammer_Impact" (0.0 0.0 0.0) (struct) (2.0 2.0 2.0))
  (`NiagaraFunctionLibrary.SpawnSystemAtLocation` "/Game/Free_Magic/VFX_Niagara/NS_Free_Magic_Area1.NS_Free_Magic_Area1" (`.Location` (`GameplayStatics.BreakHitResult` Hit)) (struct) (0.5 0.5 0.5)))

(fn `setvelocity`
  (params (target :type "Actor Object Reference"))
  (bind _newvelocity (`parent.setvelocity` target))
  (`ProjectileMovementComponent.SetVelocityInLocalSpace` (`self.ProjectileMovement`) (- _newvelocity (0.0 0.0 100.0))))

(fn `UserConstructionScript`
  (`parent.UserConstructionScript`))
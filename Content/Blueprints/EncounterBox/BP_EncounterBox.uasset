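; Encounter trigger volume that starts random battles when the player character enters its box.
; Overlap sets a one-shot timer for a random roll, where zero disables player input and adds a fade widget.
; It then spawns BP_BattleManager using randomly picked EncounterLocation transforms, passes it ChangeArray, and after short delays blends the view to it and starts its spinning camera.
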(event `self.ReceiveBeginPlay`
  (bind _asbp_third_person_character (cast `/Game/ThirdPerson/Blueprints/BP_ThirdPersonCharacter` (`GameplayStatics.GetPlayerCharacter` 0)))
  (set `self.MainCharacter` _asbp_third_person_character)
  (`self.EnableInput` (`GameplayStatics.GetPlayerController` 0)))

(event `self.Box.OnComponentBeginOverlap`
  (params (OverlappedComponent :type "PrimitiveComponent Object Reference") (OtherActor :type "Actor Object Reference") (OtherComp :type "PrimitiveComponent Object Reference") (OtherBodyIndex :type Integer) (bFromSweep :type Boolean) (SweepResult :type "HitResult Structure (by ref)"))
  (if (== OtherActor (`self.MainCharacter`))
    (`KismetSystemLibrary.K2_SetTimerDelegate` (delegate `Impulse`) (`self.Impulse Intervals`))))

(event `Key|One`
  (params (Key :type "Key Structure"))
  (:`Pressed`
    (`KismetSystemLibrary.PrintString` (`KismetStringLibrary.Conv_IntToString` (`KismetArrayLibrary.Array_Length` (`self.EncounterLocation`))))))

(event `Impulse`
  (bind _encounterlocation (`self.EncounterLocation`))
  (bind _output (`|GetArrayItem` _encounterlocation (`KismetMathLibrary.RandomIntegerInRange` 0 (- (`KismetArrayLibrary.Array_Length` _encounterlocation) 1))))
  (switch `int` (`KismetMathLibrary.RandomIntegerInRange` 0 (`self.Random Max`))
    (:`0`
      (`KismetSystemLibrary.K2_ClearTimer` null "Impulse")
      (`KismetSystemLibrary.PrintString` "StartEncounter")
      (`self.DisableInput` (`self.MainCharacter`) (`GameplayStatics.GetPlayerController` 0))
      (bind _returnvalue (`|CreateWidget` "/Game/HUD/UI_Fade.UI_Fade_C" (`GameplayStatics.GetPlayerController` 0)))
      (`UserWidget.AddToViewport` _returnvalue 0)
      (bind _returnvalue_2 (`|SpawnActorFromClass` "/Game/Blueprints/BattleManager/BP_BattleManager.BP_BattleManager_C" (`KismetMathLibrary.MakeTransform` (`SceneComponent.K2_GetComponentLocation` (`/Game/Blueprints/EncounterBox/BP_EncounterLocation.DefaultSceneRoot` _output)) (`SceneComponent.K2_GetComponentRotation` (`/Game/Blueprints/EncounterBox/BP_EncounterLocation.DefaultSceneRoot` _output))) "AlwaysSpawn" "MultiplyWithRoot" null (`self.ChangeArray`) null))
      (`KismetSystemLibrary.Delay` 1.0)
      (`PlayerController.SetViewTargetWithBlend` (`GameplayStatics.GetPlayerController` 0) _returnvalue_2 0.0 "VTBlend_Linear" 0.0 false)
      (`KismetSystemLibrary.Delay` 1.0)
      (`/Game/Blueprints/BattleManager/BP_BattleManager.TransitionToSpinningCamera` _returnvalue_2))))

(fn `UserConstructionScript`)